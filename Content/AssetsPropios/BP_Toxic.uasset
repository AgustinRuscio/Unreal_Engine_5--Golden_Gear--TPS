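; BP_Toxic is a toxic hazard area that hurts the third-person player character while it stands inside.
; Box overlap events store and clear the Player reference, switching the Plane material's WaterBaseColor to red on entry and dark green on exit.
; While that reference is valid, Tick calls GetDamage on the player's BCLifeComponent, applying Damage every frame without delta-time scaling.
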(event OnComponentEndOverlap(Box)
  (params (OverlappedComponent :type Primitive%20Component%20Object%20Reference) (OtherActor :type Actor%20Object%20Reference) (OtherComp :type Primitive%20Component%20Object%20Reference) (OtherBodyIndex :type Integer))
  (if (== OtherActor (Variables|Default|GetPlayer))
    (Variables|Default|SetPlayer 0)
    (Rendering|Material|SetVectorParameterValueonMaterials (Variables|Default|GetPlane) "WaterBaseColor" (Math|Vector|MakeVector 0.0 0.041667 0.014694))))

(event OnComponentBeginOverlap(Box)
  (params (OverlappedComponent :type Primitive%20Component%20Object%20Reference) (OtherActor :type Actor%20Object%20Reference) (OtherComp :type Primitive%20Component%20Object%20Reference) (OtherBodyIndex :type Integer) (bFromSweep :type Boolean) (SweepResult :type Hit%20Result%20Structure%20%28by%20ref%29))
  (bind _asbp_third_person_character (Utilities|Casting|CastToBP_ThirdPersonCharacter OtherActor))
  (Variables|Default|SetPlayer _asbp_third_person_character)
  (Rendering|Material|SetVectorParameterValueonMaterials (Variables|Default|GetPlane) "WaterBaseColor" (Math|Vector|MakeVector 0.385417 0.003677 0.019016)))

(event EventTick
  (params (DeltaSeconds :type Float%20%28single-precision%29))
  (Utilities|IsValid (Variables|Default|GetPlayer)
    (:Is%20Valid
      (Default|GetDamage (Variables|/Game/ThirdPerson/Blueprints/BP_ThirdPersonCharacter.BP_ThirdPersonCharacter_C|GetBC_LifeComponent (Variables|Default|GetPlayer)) (Variables|Default|GetDamage)))))

(fn ConstructionScript)