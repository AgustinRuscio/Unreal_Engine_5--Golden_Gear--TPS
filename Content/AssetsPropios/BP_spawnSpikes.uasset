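; Spawner actor that periodically creates BP_Spikes hazards at its own location.
; On BeginPlay a looping timer fires every few seconds, spawning enlarged spikes with the spawner's rotation and passing its Offset to each through SetOffest.
; Disconnected CanShoot and timeline cooldown nodes remain in the graph but never run.
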(event Custom|Spawn
  (bind _returnvalue (Game|SpawnActorfromClass "/Game/AssetsPropios/BP_Spikes.BP_Spikes_C" (Math|Transform|MakeTransform (Transformation|GetActorLocation) (Transformation|GetActorRotation) "2.000000,2.000000,2.000000") "Undefined" 0 0))
  (Default|SetOffest _returnvalue (Variables|Default|Getoffset)))

(event EventBeginPlay
  (Utilities|Time|SetTimerbyEvent (delegate Custom|Spawn) 3.0 true))

(fn ConstructionScript)