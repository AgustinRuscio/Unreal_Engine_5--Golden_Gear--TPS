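; Door actor, named for lever (palanca) use, that slides between closed and open positions through its OpenDoor and CloseDoor events.
; BeginPlay caches the start location and tints the mesh red through a material Color parameter.
; The OpenCloseDoor timeline lerps the whole actor toward start plus OpenOffset, without sweep.
; Opening changes the tint and always plays from start, while closing restores red and reverses the timeline.
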(event Custom|Open%20Door
  (bind _initiallocation (Variables|Default|GetInitialLocation))
  (Rendering|Material|SetVectorParameterValueonMaterials (Variables|Default|GetStaticMesh) "Color" (Math|Vector|MakeVector 0.358071 0.390625 0.325521))
  (bind _time (Timeline|OpenCloseDoor PlayFromStart)
    (:Update
      (Transformation|SetActorLocation (Math|Vector|Lerp(Vector) _initiallocation (+ _initiallocation (Variables|Default|GetOpenOffset)) _time) false false))))

(event Custom|Close%20Door
  (bind _initiallocation (Variables|Default|GetInitialLocation))
  (Rendering|Material|SetVectorParameterValueonMaterials (Variables|Default|GetStaticMesh) "Color" (Math|Vector|MakeVector 1.0 0.032914 0.0))
  (bind _time (Timeline|OpenCloseDoor Reverse)
    (:Update
      (Transformation|SetActorLocation (Math|Vector|Lerp(Vector) _initiallocation (+ _initiallocation (Variables|Default|GetOpenOffset)) _time) false false))))

(event EventBeginPlay
  (Variables|Default|SetInitialLocation (Transformation|GetActorLocation))
  (Rendering|Material|SetVectorParameterValueonMaterials (Variables|Default|GetStaticMesh) "Color" (Math|Vector|MakeVector 1.0 0.032914 0.0)))

(fn ConstructionScript)