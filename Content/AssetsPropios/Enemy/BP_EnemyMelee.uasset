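; BP_EnemyMelee is a melee enemy driven by a Blackboard on its controller.
; BeginPlay calls LoadValues, sets the current waypoint, then writes enemy type and damage after staggered delays.
; Perception updates write the actor, cast to the third-person character, as target, whether sensed or lost.
; On life-component death it sets the death key once, plays a montage, and destroys itself on completion.
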(event OnDeath(BC_LifeComponent)
  (if (not (Variables|Default|GetDeath))
    (bind _output_get (Variables|Default|SetDeath true))
    (AI|Components|Blackboard|SetValueasBool (AI|GetBlackboard (Pawn|GetController)) (Variables|Default|GetDeathName) _output_get)
    (Animation|Montage|PlayMontage (Variables|Character|GetMesh) "/Game/CityofBrass_Enemies/Meshes/Enemy/Corpse/animation/AM_Death.AM_Death"
      (:OnCompleted
        (Actor|DestroyActor)))))

(event OnTargetPerceptionUpdated(AIPerception)
  (params (Actor :type Actor%20Object%20Reference) (Stimulus :type AI%20Stimulus%20Structure))
  (bind _asbp_third_person_character (Utilities|Casting|CastToBP_ThirdPersonCharacter Actor))
  (AI|Components|Blackboard|SetValueasObject (AI|GetBlackboard (Pawn|GetController)) (Variables|Default|GetTargetKey) (select (.bsuccessfullysensed Stimulus) _asbp_third_person_character _asbp_third_person_character)))

(event EventBeginPlay
  (bind _returnvalue (Pawn|GetController))
  (bind _returnvalue_2 (AI|GetBlackboard _returnvalue))
  (CallFunction|LoadValues)
  (AI|Components|Blackboard|SetValueasVector _returnvalue_2 (Variables|Default|GetCurrentWaypoint) (Transformation|GetActorLocation (Utilities|Array|Get(acopy) (Variables|Default|GetWayPoints) (Variables|Default|GetwaypointIndex))))
  (Utilities|FlowControl|Delay 1.0)
  (AI|Components|Blackboard|SetValueasEnum _returnvalue_2 (Variables|Default|GetEnemyTypee) (Variables|Default|GetEnemyType))
  (Utilities|FlowControl|Delay 1.0)
  (AI|Components|Blackboard|SetValueasFloat _returnvalue_2 (Variables|Default|GetDamageKey) (Variables|Default|GetDamage)))

(fn ConstructionScript
  (CallFunction|LoadValues))