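; BP_EnemyCounterManager tracks the enemies in the level and signals when all of them are defeated.
; On BeginPlay it gathers every BP_Enemy into an array and binds an event to each one's OnDeath dispatcher.
; Its defeat handler removes the given enemy from the array and calls OnAllEnemiesDefeat once the array is empty.
; Enemies spawned after BeginPlay are not tracked.
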(event Custom|OnenemyDefeat
  (params (Enemy :type BP%20Enemy%20Object%20Reference))
  (if (Utilities|Array|ContainsItem (Variables|Default|GetAllEnemies) Enemy)
    (Utilities|Array|RemoveItem (Variables|Default|GetAllEnemies) Enemy)
    (CallFunction|CheckEnemyCount)))

(event Custom|Check%20Enemy%20Count
  (if (Utilities|Array|IsEmpty (Variables|Default|GetAllEnemies))
    (Default|CallOnAllEnemiesDefeat)))

(event EventBeginPlay
  (bind _outactors (Actor|GetAllActorsOfClass "/Game/ThirdPerson/Enemy/BP_Enemy.BP_Enemy_C"))
  (bind _output_get (Variables|Default|SetAllEnemies _outactors))
  (for _array_element _output_get
    (EventDispatchers|BindEventtoOnDeath _array_element (EventDispatchers|CreateEvent :!event Custom|OnenemyDefeat))))

(fn ConstructionScript)