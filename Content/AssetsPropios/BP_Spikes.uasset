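; BP_Spikes is a short-lived damaging spike actor that moves along an offset and hurts the third-person character on contact.
; On BeginPlay it sets a five-second lifespan, then a timeline lerps it from its starting position by Offset, which the SetOffest event can set.
; An overlap with BP_ThirdPersonCharacter applies Damage through that character's BCLifeComponent and destroys the spikes.
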(event OnComponentBeginOverlap(e)
  (params (OverlappedComponent :type Primitive%20Component%20Object%20Reference) (OtherActor :type Actor%20Object%20Reference) (OtherComp :type Primitive%20Component%20Object%20Reference) (OtherBodyIndex :type Integer) (bFromSweep :type Boolean) (SweepResult :type Hit%20Result%20Structure%20%28by%20ref%29))
  (bind _asbp_third_person_character (Utilities|Casting|CastToBP_ThirdPersonCharacter OtherActor))
  (Default|GetDamage (Variables|/Game/ThirdPerson/Blueprints/BP_ThirdPersonCharacter.BP_ThirdPersonCharacter_C|GetBC_LifeComponent _asbp_third_person_character) (Variables|Default|Getdamage))
  (Actor|DestroyActor))

(event Custom|SetOffest
  (params (NewParam :type Vector))
  (Variables|Default|Setoffset NewParam))

(event EventBeginPlay
  (Variables|Default|SetinitialPos (Transformation|GetActorLocation))
  (Actor|SetLifeSpan 5.0)
  (bind _newtrack_0 (Timeline|Timeline_0 Play)
    (:Update
      (Transformation|SetActorLocation (Math|Vector|Lerp(Vector) (Variables|Default|GetinitialPos) (+ (Variables|Default|GetinitialPos) (Variables|Default|Getoffset)) _newtrack_0) false false))))

(fn ConstructionScript)