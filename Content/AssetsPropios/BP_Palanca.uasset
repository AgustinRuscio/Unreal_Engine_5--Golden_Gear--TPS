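; BP_Palanca is a lever that the player can use to open and close a linked door.
; Overlapping its trigger shows a widget and registers the lever as the third-person character's current interactable; leaving reverses both.
; Each OBjectInteraction event flip-flops between opening and closing the door referenced by OpenedDoor.
; Both overlap events also create a dynamic material instance on the cube without changing its parameters.
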(event OnComponentBeginOverlap(r)
  (params (OverlappedComponent :type Primitive%20Component%20Object%20Reference) (OtherActor :type Actor%20Object%20Reference) (OtherComp :type Primitive%20Component%20Object%20Reference) (OtherBodyIndex :type Integer) (bFromSweep :type Boolean) (SweepResult :type Hit%20Result%20Structure%20%28by%20ref%29))
  (Rendering|Material|CreateDynamicMaterialInstance (Variables|Default|GetCube) 0 0 "None" :!class /Script/Engine.PrimitiveComponent)
  (bind _asbp_third_person_character (Utilities|Casting|CastToBP_ThirdPersonCharacter OtherActor))
  (Rendering|SetVisibility (Variables|Default|GetWidget) true false)
  (Default|SetInteractuable _asbp_third_person_character true self))

(event OnComponentEndOverlap(r)
  (params (OverlappedComponent :type Primitive%20Component%20Object%20Reference) (OtherActor :type Actor%20Object%20Reference) (OtherComp :type Primitive%20Component%20Object%20Reference) (OtherBodyIndex :type Integer))
  (Rendering|Material|CreateDynamicMaterialInstance (Variables|Default|GetCube) 0 0 "None" :!class /Script/Engine.PrimitiveComponent)
  (bind _asbp_third_person_character (Utilities|Casting|CastToBP_ThirdPersonCharacter OtherActor))
  (Rendering|SetVisibility (Variables|Default|GetWidget) false false)
  (Default|SetInteractuable _asbp_third_person_character false self))

(event EventOBjectInteraction
  (bind _openeddoor (Variables|Default|GetOpenedDoor))
  (Utilities|FlowControl|FlipFlop
    (:A
      (Default|OpenDoor _openeddoor))
    (:B
      (Default|CloseDoor _openeddoor))))

(fn ConstructionScript)