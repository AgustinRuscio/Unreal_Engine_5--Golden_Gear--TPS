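; Interactable door that the player swings open and closed while inside its trigger box.
; Box overlaps register or clear the door as the ThirdPersonCharacter's current interactable and show or hide two prompt widgets.
; The OBjectInteraction event alternates through a FlipFlop between playing and reversing a Timeline that lerps the mesh's relative yaw through a quarter turn.
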(event OnComponentBeginOverlap(Box)
  (params (OverlappedComponent :type Primitive%20Component%20Object%20Reference) (OtherActor :type Actor%20Object%20Reference) (OtherComp :type Primitive%20Component%20Object%20Reference) (OtherBodyIndex :type Integer) (bFromSweep :type Boolean) (SweepResult :type Hit%20Result%20Structure%20%28by%20ref%29))
  (bind _asbp_third_person_character (Utilities|Casting|CastToBP_ThirdPersonCharacter OtherActor))
  (Default|SetInteractuable _asbp_third_person_character true self)
  (Rendering|SetVisibility (Variables|Default|GetWidget) true false)
  (Rendering|SetVisibility (Variables|Default|GetWidget1) true false))

(event OnComponentEndOverlap(Box)
  (params (OverlappedComponent :type Primitive%20Component%20Object%20Reference) (OtherActor :type Actor%20Object%20Reference) (OtherComp :type Primitive%20Component%20Object%20Reference) (OtherBodyIndex :type Integer))
  (bind _asbp_third_person_character (Utilities|Casting|CastToBP_ThirdPersonCharacter OtherActor))
  (Default|SetInteractuable _asbp_third_person_character false self)
  (Rendering|SetVisibility (Variables|Default|GetWidget) false false)
  (Rendering|SetVisibility (Variables|Default|GetWidget1) false false))

(event EventOBjectInteraction
  (Utilities|FlowControl|FlipFlop
    (:A
      (bind _time (Timeline|Timeline_0 PlayFromStart)
        (:Update
          (Transformation|SetRelativeRotation (Variables|Default|GetStaticMesh) (Math|Rotator|MakeRotator 0.0 0.0 (Math|Float|Lerp 0.0 9e+01 _time)) false false))))
    (:B
      (Timeline|Timeline_0 Reverse))))

(fn ConstructionScript)